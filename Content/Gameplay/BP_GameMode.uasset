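; Game mode for a timed collectible game that runs the intro screen, countdown, scoring and game over.
; After a short intro widget it shows the in-game UI and starts a looping one-second timer; zero triggers game over and opens TP01_Labyrinth.
; GameDone pauses the timer and sums collectible and remaining-time points.
; Separate events save records to the instance1 GameInstance, counting more remaining seconds as a better time despite the name Lowesttime.
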(event `self.ReceiveBeginPlay`
  ;[1 1 1] Starting Level
  (bind _returnvalue (`|CreateWidget` "/Game/Gameplay/UI_DebutdeJeu.UI_DebutdeJeu_C"))
  (`UserWidget.AddToViewport` _returnvalue 0)
  (`KismetSystemLibrary.Delay` 3.0)
  (`Widget.RemoveFromParent` _returnvalue)
  (`self.GameBegin`))

(event `calculmeilleurtemps`
  (bind _second (`self.Second`))
  ;[1 1 1] Calcul du meilleur temps
  (bind _asinstance_1 (cast `/Game/Gameplay/instance1` (`GameplayStatics.GetGameInstance`)))
  (if (> (`KismetMathLibrary.Conv_IntToDouble` _second) (`/Game/Gameplay/instance1.Lowesttime` _asinstance_1))
    (set `/Game/Gameplay/instance1.Lowesttime` (`KismetMathLibrary.Conv_IntToDouble` _second) _asinstance_1)
    (set `self.new_lowtime` true)))

(event `ActivatedTimer`
  ;[1 1 1] Timer - WORKING <3
  (bind _returnvalue (`KismetSystemLibrary.K2_SetTimer` null "TimeDecrement" 1.0 true)))

(event `PausedTimer`
  ;[1 1 1] Timer - WORKING <3
  (`KismetSystemLibrary.K2_PauseTimerHandle` (stale `ActivatedTimer` _returnvalue)))

(event `AddScoreCollectibles`
  ;[1 1 1] Score Collectibles
  (set `self.ScoreCollectibles` (* (`self.NbCollectibles`) 1000)))

(event `AddScoreTime`
  ;[1 1 1] Score Timer
  (set `self.ScoreTimer` (* (`self.Second`) 50)))

(event `calculmeilleurscore`
  (bind _score (`self.Score`))
  ;[1 1 1] Calcul meilleur score
  (bind _asinstance_1 (cast `/Game/Gameplay/instance1` (`GameplayStatics.GetGameInstance`)))
  (if (>= _score (`/Game/Gameplay/instance1.Highscore` _asinstance_1))
    (set `/Game/Gameplay/instance1.Highscore` _score _asinstance_1)
    (set `self.new_highscore` true)))

(event `AddCollectibles`
  ;[1 1 1] Adding Collectibles
  (set `self.NbCollectibles` (+ (`self.NbCollectibles`) 1)))

(event `GameOver`
  ;[1 1 1] GameOver Event
  (bind _returnvalue (`|CreateWidget` "/Game/Gameplay/UI_Gameover.UI_Gameover_C"))
  (`UserWidget.AddToViewport` _returnvalue 0)
  (`KismetSystemLibrary.Delay` 3.0)
  (`GameplayStatics.OpenLevel` "TP01_Labyrinth"))

(event `GameBegin`
  ;[1 1 1] Game Begin
  (`self.ActivatedTimer`)
  (bind _returnvalue (`|CreateWidget` "/Game/Gameplay/UI_MidGame.UI_MidGame_C"))
  (`UserWidget.AddToViewport` _returnvalue 0))

(event `GameDone`
  ;[1 1 1] Calculating Score
  (`self.PausedTimer`)
  (`self.FinalScore`))

(event `FinalScore`
  ;[1 1 1] Calculate Final Score
  (`self.AddScoreCollectibles`)
  (`self.AddScoreTime`)
  (set `self.Score` (+ (`self.ScoreCollectibles`) (`self.ScoreTimer`))))

(fn `TimeDecrement`
  (bind _output_get (set `self.Second` (- (`self.Second`) 1)))
  (if (== _output_get 0)
    (`self.GameOver`)))

(fn `UserConstructionScript`)