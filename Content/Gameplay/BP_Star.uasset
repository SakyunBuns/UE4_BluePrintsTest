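; BP_Star is a level-ending goal pickup for a labyrinth game, marked in its graph as deprecated or due for a remake.
; Overlapping its box pauses the game mode timer, plays a victory sound and moves the star vertically on a timeline.
; When the timeline finishes, it toggles the star's visibility, has BP_GameMode end the game and compute best time and score, shows the end-game widget, then opens TP01_Labyrinth after a delay.
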(event `self.Box.OnComponentBeginOverlap`
  (params (OverlappedComponent :type "PrimitiveComponent Object Reference") (OtherActor :type "Actor Object Reference") (OtherComp :type "PrimitiveComponent Object Reference") (OtherBodyIndex :type Integer) (bFromSweep :type Boolean) (SweepResult :type "HitResult Structure (by ref)"))
  ;[1 1 1] Debricated or should be remade
  (bind _asbp_game_mode (cast `/Game/Gameplay/BP_GameMode` (`GameplayStatics.GetGameMode`)))
  (`/Game/Gameplay/BP_GameMode.PausedTimer` _asbp_game_mode)
  (`GameplayStatics.PlaySoundAtLocation` "/Game/Assets/165491__chripei__victory-cry-reverb-2.165491__chripei__victory-cry-reverb-2" (`SceneComponent.K2_GetComponentLocation` (`Actor.RootComponent` (`GameplayStatics.GetPlayerCharacter` 0))) (struct) 1.0 1.0 0.0 null null null)
  (bind (_direction _newtrack_0) (`Timeline|Timeline_0`)
    (:`Update`
      (`SceneComponent.K2_SetRelativeLocation` (`self.Star`) (`KismetMathLibrary.MakeVector` 0.0 0.0 _newtrack_0) false false))
    (:`Finished`
      (`SceneComponent.ToggleVisibility` (`self.Star`) true)
      (bind _asbp_game_mode_2 (cast `/Game/Gameplay/BP_GameMode` (`GameplayStatics.GetGameMode`)))
      (`/Game/Gameplay/BP_GameMode.GameDone` _asbp_game_mode_2)
      (`/Game/Gameplay/BP_GameMode.calculmeilleurtemps` _asbp_game_mode_2)
      (`/Game/Gameplay/BP_GameMode.calculmeilleurscore` _asbp_game_mode_2)
      (bind _returnvalue (`|CreateWidget` "/Game/Gameplay/UI_FindeJeu.UI_FindeJeu_C"))
      (bind _output_get (set `self.REF_Ecran` _returnvalue))
      (`UserWidget.AddToViewport` _output_get 0)
      (`KismetSystemLibrary.Delay` 5.0)
      (`GameplayStatics.OpenLevel` "TP01_Labyrinth"))))

(fn `UserConstructionScript`)