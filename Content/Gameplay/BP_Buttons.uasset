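; One-shot push button the player activates by input while inside its collision volume, which also shows a "Press B" widget.
; Pressing it increments the game mode's switch count, swaps the material to activated and plays a cowbell at the player.
; A timeline moves the button along Z, calling DoorOpen on all BP_Door actors found via GetAllActorsOfClass on every update tick.
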(event `InputAction|Button_Activation`
  (params (Key :type "Key Structure"))
  ;[1 1 1] Button_Activate
  (:`Pressed`
    (`/Engine/EditorBlueprintResources/StandardMacros.DoOnce` false
      (:`Completed`
        (`|ExecutionSequence`
          (:`then_0`
            (`self.Interrupteurs_Update`)
            (bind (_direction _postion_z) (`Timeline|Animation_Button`)
              (:`Update`
                (`SceneComponent.K2_SetRelativeLocation` (`self.Button_Button`) (`KismetMathLibrary.MakeVector` 0.0 0.0 _postion_z) false false)
                (bind _outactors (`GameplayStatics.GetAllActorsOfClass` "/Game/Gameplay/BP_Door.BP_Door_C"))
                (`/Game/Gameplay/BP_Door.Door_Open` _outactors))))
          (:`then_1`
            (`PrimitiveComponent.SetMaterial` (`self.Button_Button`) 0 "/Game/Gameplay/Materials/M_Activated.M_Activated"))
          (:`then_2`
            (`GameplayStatics.PlaySoundAtLocation` "/Game/Assets/Cartoon_Cowbell.Cartoon_Cowbell" (`SceneComponent.K2_GetComponentLocation` (`Actor.RootComponent` (`GameplayStatics.GetPlayerCharacter` 0))) (struct) 1.0 1.0 0.0 null null null)))))))

(event `self.Button_Collision.OnComponentBeginOverlap`
  (params (OverlappedComponent :type "PrimitiveComponent Object Reference") (OtherActor :type "Actor Object Reference") (OtherComp :type "PrimitiveComponent Object Reference") (OtherBodyIndex :type Integer) (bFromSweep :type Boolean) (SweepResult :type "HitResult Structure (by ref)"))
  ;[1 1 1] Button_EnteringCollision
  (`self.EnableInput` (`GameplayStatics.GetPlayerController` 0))
  (bind _returnvalue (`|CreateWidget` "/Game/Gameplay/UI_PressB_Display.UI_PressB_Display_C"))
  (bind _output_get (set `self.PressBDisplay` _returnvalue))
  (`UserWidget.AddToViewport` _output_get 0))

(event `self.Button_Collision.OnComponentEndOverlap`
  (params (OverlappedComponent :type "PrimitiveComponent Object Reference") (OtherActor :type "Actor Object Reference") (OtherComp :type "PrimitiveComponent Object Reference") (OtherBodyIndex :type Integer))
  ;[1 1 1] Button_EnteringCollision
  (`self.DisableInput` (`GameplayStatics.GetPlayerController` 0))
  (`Widget.RemoveFromParent` (`self.PressBDisplay`)))

(event `Interrupteurs_Update`
  ;[1 1 1] Interrupteur_UpdateNumber
  (bind _asbp_game_mode (cast `/Game/Gameplay/BP_GameMode` (`GameplayStatics.GetGameMode`)))
  (set `/Game/Gameplay/BP_GameMode.NbInterrupteurs` (+ (`/Game/Gameplay/BP_GameMode.NbInterrupteurs` _asbp_game_mode) 1) _asbp_game_mode))

(event `Button_ColorChange`
  (params (Color_Red :type "Color Structure"))
  (`MeshComponent.SetVectorParameterValueOnMaterials` (`self.Button_Button`) "M_Activated" (0.0 0.0 0.0)))

(fn `UserConstructionScript`
  (bind _returnvalue (`PrimitiveComponent.CreateDynamicMaterialInstance` (`self.Button_Button`) 0 "/Game/Gameplay/Materials/M_UnActive.M_Unactive" "None"))
  (set `self.Button_Color` _returnvalue))