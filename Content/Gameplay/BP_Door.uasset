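; Door actor that slides open once every switch in the level has been activated.
; Its Door_Open event checks whether the switch count in BP_GameMode equals the maximum and does nothing otherwise.
; On a match it plays a deadbolt sound at the player character's location, then a timeline drives the door component's relative location.
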(event `Door_Open`
  ;[1 1 1] Door_TranslateZ
  (bind _asbp_game_mode (cast `/Game/Gameplay/BP_GameMode` (`GameplayStatics.GetGameMode`)))
  (if (== (`/Game/Gameplay/BP_GameMode.NbInterrupteurs` _asbp_game_mode) (`/Game/Gameplay/BP_GameMode.NbMaxInterrupteurs` _asbp_game_mode))
    (`GameplayStatics.PlaySoundAtLocation` "/Game/Assets/Deadbolt_Lock.Deadbolt_Lock" (`SceneComponent.K2_GetComponentLocation` (`Actor.RootComponent` (`GameplayStatics.GetPlayerCharacter` 0))) (struct) 1.0 1.0 0.0 null null null)
    (bind (_direction _door_translatez) (`Timeline|Door_Animation`)
      (:`Update`
        (`SceneComponent.K2_SetRelativeLocation` (`self.Door`) _door_translatez false false)))))

(fn `UserConstructionScript`)